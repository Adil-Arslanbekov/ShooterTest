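; BP_WeaponBase is a base weapon actor that loads its settings from a DT_Weapon row at construction and fires bullets.
; Press and release events drive a gate that, in Auto mode, loops on a retriggerable FireRate delay.
; Each shot plays the AK47 montage and spawns a Bullet at the muzzle, rotated by a visibility trace.
; Spread is loaded but not applied, and the trace's hit normal, not impact point, serves as aim target.
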(event `StartFire`
  (switch `/Game/Blueprints/BP_Weapon/Enum_FireMode` (`self.FireMode`)
    (:`NewEnumerator2`
      (`|ExecutionSequence`
        (:`then_0`
          (goto _label :!via `Open`))
        (:`then_1`
          (`/Engine/EditorBlueprintResources/StandardMacros.Gate` true :!label _label
            (:`Exit`
              (`|ExecutionSequence`
                (:`then_0`
                  (`KismetSystemLibrary.RetriggerableDelay` (`self.FireRate`))
                  (goto _label))
                (:`then_1`
                  (`self.SpawnProjectile`)
                  (`KismetSystemLibrary.PrintString` "Fired" true true (struct :`G` 0.66 :`B` 1.0 :`A` 1.0) 0.5))))))))))

(event `StopFire`
  (goto _label :!via `Close`))

(event `FirePress`
  (`self.StartFire`))

(event `FireRelease`
  (`self.StopFire`))

(event `self.ReceiveBeginPlay`
  (`KismetSystemLibrary.Delay` 0.2)
  (`KismetSystemLibrary.PrintString` (`KismetStringLibrary.Conv_NameToString` (`self.MuzzleName`))))

(fn `CalculateDirection`
  (returns (Location :type "Vector Structure") (Rotation :type "Rotator Structure"))
  (bind _returnvalue (`self.MuzzlePosition`))
  (bind _charref (`self.CharRef`))
  (bind (_returnvalue_location _returnvalue_rotation) (`KismetMathLibrary.BreakTransform` (`SceneComponent.K2_GetComponentToWorld` (`Actor.RootComponent` (select `bool` (`/Game/Blueprints/BP_PlayerCharacter.Aiming` _charref) :`true` _charref)))))
  (bind _returnvalue_2 (+ _returnvalue_location (* (`KismetMathLibrary.GetForwardVector` _returnvalue_rotation) 10000.0)))
  (bind (_outhit _returnvalue_3) (`KismetSystemLibrary.LineTraceSingle` :`Start` (+ _returnvalue_location (* (`KismetMathLibrary.GetForwardVector` _returnvalue_rotation) (`KismetMathLibrary.VSize` (- _returnvalue_location (`self.MuzzlePosition`))))) :`End` _returnvalue_2 :`TraceChannel` "TraceTypeQuery1" :`DrawDebugType` "ForDuration"))
  (return _returnvalue (`KismetMathLibrary.FindLookAtRotation` _returnvalue (`KismetMathLibrary.SelectVector` (`.ImpactNormal` (`GameplayStatics.BreakHitResult` _outhit)) _returnvalue_2 _returnvalue_3))))

(fn `CalculateFinalDirection`
  (params (Location :type "Vector Structure") (Rotation :type "Rotator Structure"))
  (returns (Transform :type "Transform Structure"))
  (return (`KismetMathLibrary.MakeTransform` Location (`KismetMathLibrary.ComposeRotators` Rotation (`KismetMathLibrary.MakeRotator` 0.0)))))

(fn `SpawnProjectile`
  (`AnimInstance.Montage_Play` (`SkeletalMeshComponent.GetAnimInstance` (`self.AK47`)) "/Game/Anim/Weapon/KA47_Shoot_Montage.KA47_Shoot_Montage" 1.0 "MontageLength" 0.0 true)
  (bind (_location _rotation) (`self.CalculateDirection`))
  (bind _transform (`self.CalculateFinalDirection` _location _rotation))
  (`|SpawnActorFromClass` "/Game/Blueprints/BP_Weapon/Bullet.Bullet_C" _transform "Undefined" "OverrideRootScale" null null))

(fn `UserConstructionScript`
  (bind _returnvalue (`|GetDataTableRow` "/Game/Blueprints/BP_Weapon/DT_Weapon.DT_Weapon" (`self.WeaponRownName`))
    (:`then`
      (bind _output_get (set `self.WeaponData` _returnvalue))
      (bind (_firemode _muzzlename _firerate _reloaddelay _weaponspread) (break `/Game/Blueprints/BP_Weapon/Struct_WeaponData` _output_get))
      (set `self.FireMode` _firemode)
      (set `self.MuzzleName` _muzzlename)
      (set `self.FireRate` _firerate)
      (set `self.ReloadDelay` _reloaddelay)
      (set `self.WeaponSpread` _weaponspread))))